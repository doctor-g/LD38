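; BP_Planet is a planet actor that pulls every BP_PlayerShip in the level toward its Sphere component.
; Each Tick it finds all ships and adds linear physics velocity to each SPPlayerShip component, aimed at the sphere via a look-at rotation.
; The pull follows an inverse-square falloff, Gravity divided by squared distance, and is applied per frame without delta-time scaling.
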(event `self.ReceiveTick`
  (params (DeltaSeconds :type "Float (single-precision)"))
  (bind _returnvalue (`SceneComponent.K2_GetComponentLocation` (`self.Sphere`)))
  (bind _outactors (`GameplayStatics.GetAllActorsOfClass` "/Game/Characters/BP_PlayerShip.BP_PlayerShip_C"))
  (for _array_element _outactors
    (bind _sp_playership (`/Game/Characters/BP_PlayerShip.SP_PlayerShip` _array_element))
    (bind _returnvalue_2 (`SceneComponent.K2_GetComponentLocation` _sp_playership))
    (`PrimitiveComponent.SetPhysicsLinearVelocity` _sp_playership (* (`KismetMathLibrary.GetForwardVector` (`KismetMathLibrary.FindLookAtRotation` _returnvalue_2 _returnvalue)) (/ (`self.Gravity`) (`KismetMathLibrary.VSizeSquared` (- _returnvalue_2 _returnvalue)))) true "None")))

(fn `UserConstructionScript`)