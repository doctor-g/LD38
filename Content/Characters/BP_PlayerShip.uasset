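; Player ship actor that flies with physics, fires torpedoes and takes collision damage.
; Turn and thrust events apply torque and force to the sprite, while firing spawns a rotated BP_Torpedo at the Cannon socket, limited by a cooldown ticked down each frame.
; Hit speed sets damage to Health.
; At zero health the ship hides and plays an explosion flipbook, then shows the GameOver widget and pauses the game.
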(event `self.ReceiveHit`
  (params (MyComp :type "PrimitiveComponent Object Reference") (Other :type "Actor Object Reference") (OtherComp :type "PrimitiveComponent Object Reference") (bSelfMoved :type Boolean) (HitLocation :type "Vector Structure") (HitNormal :type "Vector Structure") (NormalImpulse :type "Vector Structure") (Hit :type "HitResult Structure (by ref)"))
  ;[1 1 1] Take damage on collision based on speed
  (bind _returnvalue (`PrimitiveComponent.GetPhysicsLinearVelocity` MyComp "None"))
  (`self.Take Damage` (`KismetMathLibrary.VSize` _returnvalue)))

(event `Explode`
  ;[1 1 1] Blow up the ship, removing the explosion and ship when it's all over
  (bind _returnvalue (`AddComponent|NODE_AddPaperFlipbookComponent-2`))
  (`PaperFlipbookComponent.SetLooping` _returnvalue false)
  (add `PaperFlipbookComponent.OnFinishedPlaying` _returnvalue (delegate `OnFinishedPlaying_Event_0`))
  (`SceneComponent.SetVisibility` (`self.SP_PlayerShip`) false false)
  (`AudioComponent.Play` (`self.explosion`) 0.0))

(event `OnFinishedPlaying_Event_0`
  ;[1 1 1] Blow up the ship, removing the explosion and ship when it's all over
  (`ActorComponent.K2_DestroyComponent` (stale `Explode` _returnvalue))
  (`self.Show Game Over Screen`)
  (`GameplayStatics.SetGamePaused` true))

(event `self.ReceiveBeginPlay`)

(event `Fire`
  ;[1 1 1] Fire!
  (if (== (`self.CooldownTimer`) 0.0)
    (`AudioComponent.Play` (`self.laser`) 0.0)
    (bind _returnvalue (`|SpawnActorFromClass` "/Game/Characters/BP_Torpedo.BP_Torpedo_C" (`SceneComponent.GetSocketTransform` (`self.SP_PlayerShip`) "Cannon" "RTS_World") "Undefined" "OverrideRootScale" self))
    (`self.K2_SetActorRotation` _returnvalue (`KismetMathLibrary.ComposeRotators` (struct :`Pitch` 90.0) (`self.K2_GetActorRotation`)) false)
    (set `self.CooldownTimer` (`self.FireCooldown`))))

(event `TurnLeft`
  ;[1 1 1] Handle Turn
  (`PrimitiveComponent.AddTorque` (`self.SP_PlayerShip`) (`KismetMathLibrary.MakeVector` 0.0 (- 0.0 (`self.TurnPower`))) "None" true))

(event `TurnRight`
  ;[1 1 1] Handle Turn
  (`PrimitiveComponent.AddTorque` (`self.SP_PlayerShip`) (`KismetMathLibrary.MakeVector` 0.0 (`self.TurnPower`)) "None" true))

(event `Thrust`
  (bind _sp_playership (`self.SP_PlayerShip`))
  ;[1 1 1] Handle Thrust
  (`PrimitiveComponent.AddForce` _sp_playership (`KismetMathLibrary.GreaterGreater_VectorRotator` (`KismetMathLibrary.MakeVector` 0.0 0.0 (`self.ThrustPower`)) (`SceneComponent.K2_GetComponentRotation` _sp_playership)) "None" true))

(event `self.ReceiveTick`
  (params (DeltaSeconds :type "Float (single-precision)"))
  ;[1 1 1] Update cooldown timer
  (set `self.CooldownTimer` (`KismetMathLibrary.FMax` (- (`self.CooldownTimer`) DeltaSeconds))))

(fn `Show Game Over Screen`
  (bind _returnvalue (`|CreateWidget` "/Game/UI/GameOver.GameOver_C" (`GameplayStatics.GetPlayerController` 0)))
  (`UserWidget.AddToViewport` _returnvalue 0))

(fn `Take Damage`
  (params (Amount :type "Float (double-precision)"))
  (switch `/Game/Characters/StateEnum` (`self.State`)
    (:`NewEnumerator0`
      (bind _output_get (set `self.Health` (`KismetMathLibrary.FMax` (- (`self.Health`) Amount))))
      (if (<= _output_get 0.0)
        (set `self.State` "NewEnumerator1")
        (`self.Explode`)))))

(fn `UserConstructionScript`
  (`PaperSpriteComponent.SetSprite` (`self.SP_PlayerShip`) (`self.Sprite`)))